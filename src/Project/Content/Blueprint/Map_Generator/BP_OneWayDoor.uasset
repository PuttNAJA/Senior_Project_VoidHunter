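; BP_OneWayDoor is a map generator door actor that raises its Door component while the player is inside its Trigger volume.
; BeginPlay caches the first player's BP_PlayerCharacter, and both overlap events respond only to that actor.
; Entering the trigger instantly moves the Door up by a fixed relative Z offset, and leaving moves it back down, with no interpolation.
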(event OnComponentBeginOverlap(Trigger)
  (params (OverlappedComponent :type Primitive%20Component%20Object%20Reference) (OtherActor :type Actor%20Object%20Reference) (OtherComp :type Primitive%20Component%20Object%20Reference) (OtherBodyIndex :type Integer) (bFromSweep :type Boolean) (SweepResult :type Hit%20Result%20Structure%20%28by%20ref%29))
  (bind _door (Variables|Default|GetDoor))
  (bind _relativelocation (Variables|/Script/Engine.SceneComponent|GetRelativeLocation _door))
  (if (== OtherActor (Variables|Default|GetPlayer%20Character))
    (Transformation|SetRelativeLocation (Variables|Default|GetDoor) (Math|Vector|MakeVector (.x _relativelocation) (.y _relativelocation) (+ (.z _relativelocation) 7e+02)) false false)))

(event OnComponentEndOverlap(Trigger)
  (params (OverlappedComponent :type Primitive%20Component%20Object%20Reference) (OtherActor :type Actor%20Object%20Reference) (OtherComp :type Primitive%20Component%20Object%20Reference) (OtherBodyIndex :type Integer))
  (bind _door (Variables|Default|GetDoor))
  (bind _relativelocation (Variables|/Script/Engine.SceneComponent|GetRelativeLocation _door))
  (if (== OtherActor (Variables|Default|GetPlayer%20Character))
    (Transformation|SetRelativeLocation (Variables|Default|GetDoor) (Math|Vector|MakeVector (.x _relativelocation) (.y _relativelocation) (+ (.z _relativelocation) -7e+02)) false false)))

(event EventBeginPlay
  (bind _asbp_player_character (Utilities|Casting|CastToBP_PlayerCharacter (Game|GetPlayerCharacter 0)))
  (Variables|Default|SetPlayer%20Character _asbp_player_character))

(fn ConstructionScript)