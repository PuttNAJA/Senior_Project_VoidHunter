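; Seeded procedural dungeon generator that builds a level from random room Blueprints, starting at a start room.
; Rooms attach to random open exits; after a short delay, overlap boxes reject colliding rooms and retry.
; Once the room count is met, unused exits are sealed and doors spawn at connections.
; A looping timer opens BR_Normal01 if generation exceeds the time limit; the alien spawn event is never called.
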(event Custom|Create%20Start%20Room
  ;[0.115 1 0.294 1 30] Spawn Start Room
  (bind _returnvalue (Game|SpawnActorfromClass "/Game/Blueprint/Map_Generator/BP_StartRoom.BP_StartRoom_C" (Transformation|GetWorldTransform (Variables|Default|GetDefaultSceneRoot)) "AlwaysSpawn" "MultiplyWithRoot" 0 0))
  (Utilities|Array|AppendArray (Variables|Default|GetExits%20List) (Components|GetChildrenComponents (Variables|/Game/Blueprint/Map_Generator/BP_MasterRoom.BP_MasterRoom_C|GetExits_Floder _returnvalue) false)))

(event Custom|Create%20Next%20Room
  ;[0.115 1 0.294 1 30] Spawn Next Room
  (Variables|Default|SetSelected%20Exit (.OutItem (Utilities|Array|RandomFromStream (Variables|Default|GetExits%20List) (Variables|Default|GetStream))))
  (bind _returnvalue (Game|SpawnActorfromClass (.OutItem (Utilities|Array|RandomFromStream (Variables|Default|GetRoom%20List) (Variables|Default|GetStream))) (Transformation|GetWorldTransform (Variables|Default|GetSelected%20Exit)) "AlwaysSpawn" "MultiplyWithRoot" 0 0))
  (bind _asbp_master_room (Utilities|Casting|CastToBP_MasterRoom _returnvalue))
  (Variables|Default|SetLatest%20Room _asbp_master_room)
  (Utilities|FlowControl|Delay 0.2)
  (CallFunction|CheckforOverlap))

(event Custom|Spawn%20Door
  ;[0.115 1 0.294 1 31] Create Door
  (for _array_element (Variables|Default|GetDoor%20Point%20List)
    (Game|SpawnActorfromClass (.OutItem (Utilities|Array|RandomFromStream (Variables|Default|GetDoor%20Actor%20List) (Variables|Default|GetStream))) (Transformation|GetWorldTransform _array_element) "AlwaysSpawn" "MultiplyWithRoot" 0 0)))

(event Custom|Add%20OverlapingRoom%20to%20List
  ;[0.115 1 0.294 1 30] Check for Overlap Room
  (for _array_element (Components|GetChildrenComponents (Variables|/Game/Blueprint/Map_Generator/BP_MasterRoom.BP_MasterRoom_C|GetOverlapFloder (Variables|Default|GetLatest%20Room)) false)
    (bind _asbox_collision (Utilities|Casting|CastToBoxComponent _array_element))
    (Utilities|Array|AppendArray (Variables|Default|GetOverlapped%20List) (Class|PrimitiveComponent|GetOverlappingComponents _asbox_collision))))

(event Custom|Check%20for%20Overlap
  ;[0.115 1 0.294 1 30] Delete lastest Room if Overlap
  (CallFunction|AddOverlapingRoomtoList)
  (if (Utilities|Array|IsNotEmpty (Variables|Default|GetOverlapped%20List))
    (Utilities|Array|Clear (Variables|Default|GetOverlapped%20List))
    (Actor|DestroyActor (Variables|Default|GetLatest%20Room))
    (CallFunction|CreateNextRoom)
    (else
      (Utilities|Array|Clear (Variables|Default|GetOverlapped%20List))
      (Variables|Default|SetRoom%20Amount (- (Variables|Default|GetRoom%20Amount) 1))
      (Utilities|Array|RemoveItem (Variables|Default|GetExits%20List) (Variables|Default|GetSelected%20Exit))
      ;;[1 1 1] Add to Door list
      (Utilities|Array|Add (Variables|Default|GetDoor%20Point%20List) (Variables|Default|GetSelected%20Exit))
      (Utilities|Array|AppendArray (Variables|Default|GetExits%20List) (Components|GetChildrenComponents (Variables|/Game/Blueprint/Map_Generator/BP_MasterRoom.BP_MasterRoom_C|GetExits_Floder (Variables|Default|GetLatest%20Room)) false))
      (CallFunction|AddSpawnPointtoList)
      (if (> (Variables|Default|GetRoom%20Amount) 0)
        (CallFunction|CreateNextRoom)
        (Development|PrintString "Generate Room")
        (else
          (CallFunction|CloseDoor)
          (CallFunction|SpawnDoor)
          (Variables|Default|SetDungeon_Complete true)
          (Utilities|Time|ClearandInvalidateTimerbyHandle (Variables|Default|GetTimer%20Handle))
          (Development|PrintString "Create Complete" true true "(R=0.990895,G=1.000000,B=0.000000,A=1.000000)" 1e+01))))))

(event Custom|Close%20Door
  ;[0.115 1 0.294 1 30] Close Unuse Hole
  (for _array_element (Variables|Default|GetExits%20List)
    (Game|SpawnActorfromClass "/Game/Blueprint/Map_Generator/BP_ClosedDoor.BP_ClosedDoor_C" (Transformation|GetWorldTransform _array_element) "AlwaysSpawn" "MultiplyWithRoot" 0 0)))

(event Custom|Start%20Generate%20Room%20Timer
  ;[0.115 1 0.294 1 30] Dungeon Room Timer
  (bind _returnvalue (Utilities|Time|SetTimerbyEvent (delegate Custom|Check%20Room%20Complete) 1.0 true))
  (Variables|Default|SetTimer%20Handle _returnvalue))

(event Custom|Check%20Room%20Complete
  ;[0.115 1 0.294 1 30] Dungeon Room Timer
  (Development|PrintString "Running Timer")
  (if (>= (Utilities|Time|GetGameTimeinSeconds) (Variables|Default|GetMax%20Generate%20Dungeon%20Time))
    (Game|OpenLevel(byName) "BR_Normal01")))

(event Custom|Set%20Seed
  ;[1 1 1] Set Seed, if -1 Random
  (if (== (Variables|Default|GetSeed) -1)
    (Class|KismetMathLibrary|SeedRandomStream (Variables|Default|GetStream))
    (else
      (Math|Random|SetRandomStreamSeed (Variables|Default|GetStream) (Variables|Default|GetSeed)))))

(event Custom|Add%20Spawn%20Point%20to%20List
  ;[1 1 1 1 30] Add Floor SpawnPoint To List
  (Utilities|Array|AppendArray (Variables|Default|GetFloor%20Spwan%20List) (Components|GetChildrenComponents (Variables|/Game/Blueprint/Map_Generator/BP_MasterRoom.BP_MasterRoom_C|GetFloor_SpawnPoint (Variables|Default|GetLatest%20Room)) false)))

(event Custom|Spawn%20Health%20at%20location
  ;[1 1 1 1 30] Spawn ... At location
  (if (not (<= (Variables|Default|GetHealth%20Amount) 0)) :!label _label
    (bind _output_get (Variables|Default|SetSelect%20FloorSpawn%20Location (.OutItem (Utilities|Array|RandomFromStream (Variables|Default|GetFloor%20Spwan%20List) (Variables|Default|GetStream)))))
    (Game|SpawnActorfromClass "/Game/Blueprint/Character/Enemy_01/BP_Alien_01.BP_Alien_01_C" (Math|Transform|MakeTransform (Transformation|GetWorldLocation _output_get) "0, 0, 0" "1.000000,1.000000,1.000000") "AlwaysSpawn" "MultiplyWithRoot" 0 0)
    (Utilities|Array|RemoveItem (Variables|Default|GetFloor%20Spwan%20List) (Variables|Default|GetSelect%20FloorSpawn%20Location))
    (Variables|Default|SetHealth%20Amount (- (Variables|Default|GetHealth%20Amount) 1))
    (goto _label)))

(event EventBeginPlay
  (CallFunction|SetSeed)
  (CallFunction|CreateStartRoom)
  (CallFunction|StartGenerateRoomTimer)
  (CallFunction|CreateNextRoom))

(fn ConstructionScript)