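; BP_EndRoom is the end room of the map generator, where the player triggers a spawn and clears the game.
; The first player overlap with SpawnTrigger calls Spawn, gated by a DoOnce so it runs only once.
; A player overlap with the EndGame trigger calls NMClear on the player character, with no once-only gate.
; BeginPlay and the construction script only call their parent versions.
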(event OnComponentBeginOverlap(SpawnTrigger)
  (params (OverlappedComponent :type Primitive%20Component%20Object%20Reference) (OtherActor :type Actor%20Object%20Reference) (OtherComp :type Primitive%20Component%20Object%20Reference) (OtherBodyIndex :type Integer) (bFromSweep :type Boolean) (SweepResult :type Hit%20Result%20Structure%20%28by%20ref%29))
  (if (== OtherActor (Variables|Default|GetPlayer%20Character))
    (Utilities|FlowControl|DoOnce false
      (:Completed
        (CallFunction|Spawn)))))

(event OnComponentBeginOverlap(EndGame)
  (params (OverlappedComponent :type Primitive%20Component%20Object%20Reference) (OtherActor :type Actor%20Object%20Reference) (OtherComp :type Primitive%20Component%20Object%20Reference) (OtherBodyIndex :type Integer) (bFromSweep :type Boolean) (SweepResult :type Hit%20Result%20Structure%20%28by%20ref%29))
  (if (== OtherActor (Variables|Default|GetPlayer%20Character))
    (Default|NMClear (Variables|Default|GetPlayer%20Character))))

(event EventBeginPlay
  (|CallParentFunction))

(fn ConstructionScript
  (|CallParentFunction))