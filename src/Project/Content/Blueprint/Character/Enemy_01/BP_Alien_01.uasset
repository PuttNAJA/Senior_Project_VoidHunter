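; BP_Alien_01 is an enemy alien character that punches the player and awards score and loot on death.
; Attack plays a punch montage whose notify triggers a debug-drawn sphere overlap damaging the player, then signals attack end.
; Incoming damage reduces health until Death drops a random health or ammo pickup at a downward trace hit, adds score and destroys the actor.
; SetMovementSpeed maps movement states to walk speeds.
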(event Custom|DealDamage
  (bind _attacksphere (Variables|Default|GetAttackSphere))
  (bind _returnvalue (Transformation|GetWorldLocation _attacksphere))
  ;[0.115 1 0.294 1 30] DealDamage
  (bind _outactors (Collision|SphereOverlapActors _returnvalue (Variables|Default|GetAttackRange) (Utilities|Array|MakeArray "ObjectTypeQuery3") "/Game/Blueprint/Character/Player/BP_PlayerCharacter.BP_PlayerCharacter_C" (Utilities|Array|MakeArray self)))
  (Rendering|Debug|DrawDebugSphere _returnvalue (Variables|Default|GetAttackRange) 12 "(R=1.000000,G=0.000000,B=0.178982,A=1.000000)" 2.0)
  (for _array_element _outactors
    (Game|Damage|ApplyDamage _array_element (Variables|Default|GetDamage) (Pawn|GetController) self "/Script/Engine.DamageType")))

(event Custom|Attack
  ;[0.115 1 0.294 1 30] Attack
  (Animation|Montage|PlayMontage (Variables|Default|Getenemy_01) "/Game/Animation/RamsterZ_FreeAnims_Volume1/UseAnimation/EN_PunchCombo02_Montage.EN_PunchCombo02_Montage" 1.25
    (:OnCompleted
      (Development|PrintString "Attacking" :!label _label)
      (Default|CallOnAttackEnd))
    (:OnInterrupted
      (goto _label))
    (:OnNotifyBegin
      (CallFunction|DealDamage))))

(event Custom|Drop%20loot
  (bind _returnvalue (Transformation|GetActorLocation))
  ;[0.115 1 0.294 1 30] Drop Loot
  (bind _outhit (Collision|LineTraceByChannel _returnvalue (- _returnvalue "0.000000,0.000000,200.000000") "TraceTypeQuery1" false (Utilities|Array|MakeArray (Game|GetPlayerCharacter 0)) "None"))
  (Game|SpawnActorfromClass (Utilities|Select :Index (Math|Random|RandomInteger 4) :Option%200 "/Game/Blueprint/Collected/BP_Collectable_Health.BP_Collectable_Health_C" :Option%201 "/Game/Blueprint/Collected/BP_Collectable_AR_Ammo.BP_Collectable_AR_Ammo_C" :Option%202 "/Game/Blueprint/Collected/BP_Collectable_Pistol_Ammo.BP_Collectable_Pistol_Ammo_C" :Option%203 "/Game/Blueprint/Collected/BP_Collectable_SMG_Ammo.BP_Collectable_SMG_Ammo_C" :Option%204 0) (Math|Transform|MakeTransform (.Location (Collision|BreakHitResult _outhit)) (Math|Rotator|MakeRotator 0.0 0.0 (Math|Random|RandomFloatinRange 0.0 3.6e+02)) "2.000000,2.000000,2.000000") "AdjustIfPossibleButAlwaysSpawn" "MultiplyWithRoot" 0 0)
  (Development|PrintString "Droped"))

(event Custom|Death
  ;[0.115 1 0.294 1 30] Death
  (for _index (range 0 (Math|Random|RandomInteger 0))
    (CallFunction|DropLoot))
  (bind _asbp_player_character (Utilities|Casting|CastToBP_PlayerCharacter (Game|GetPlayerCharacter 0)))
  (Default|AddScore _asbp_player_character (Variables|Default|GetDropScore))
  (Actor|DestroyActor))

(event EventBeginPlay
  (Variables|Default|SetCurrentHealth (Variables|Default|GetMaxHealth)))

(event Game|Damage|EventAnyDamage
  (params (Damage :type Float%20%28single-precision%29) (DamageType :type Damage%20Type%20Object%20Reference) (InstigatedBy :type Controller%20Object%20Reference) (DamageCauser :type Actor%20Object%20Reference))
  ;[0.115 1 0.294 1 30] Take Damage + Check Death
  (bind _output_get (Variables|Default|SetCurrentHealth (Math|Float|Truncate (- (Variables|Default|GetCurrentHealth) Damage))))
  (if (<= _output_get 0)
    (CallFunction|Death)))

(fn ConstructionScript)

(fn SetMovementSpeed
  (params (Speed :type E_MovementSpeed%20Enum :default "NewEnumerator0"))
  (bind _output_get (Variables|/Script/Engine.CharacterMovementComponent|SetMaxWalkSpeed (Variables|Character|GetCharacterMovement) (Utilities|Select :Index Speed :NewEnumerator0 0.0 :NewEnumerator1 5e+02 :NewEnumerator2 1e+03 :NewEnumerator3 1e+03)))
  (return _output_get))